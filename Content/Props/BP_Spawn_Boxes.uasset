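; Spawner prop that scatters a batch of damagable or non-damagable boxes around its location when play begins.
; A loop driven by Number spawns the class picked by IsDamagable, with random rotation and the Scale variable, always spawning despite collisions.
; Positions are random within half the actor's scale, read directly as world units, around its location.
; The lower Z bound uses Y scale instead of Z.
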(event EventBeginPlay
  (bind _returnvalue (Math|Random|RandomRotator true))
  (bind _returnvalue_2 (Transformation|GetActorLocation))
  (bind _returnvalue_3 (Transformation|GetActorScale3D))
  (bind _scale (Variables|Default|GetScale))
  (bind _returnvalue_4 (/ (.x _returnvalue_3) 2.0))
  (bind _returnvalue_5 (/ (.y _returnvalue_3) 2.0))
  (bind _returnvalue_6 (/ (.z _returnvalue_3) 2.0))
  (bind _returnvalue_7 (- (.z _returnvalue_2) _returnvalue_5))
  (bind _returnvalue_8 (+ (.z _returnvalue_2) _returnvalue_6))
  (bind _returnvalue_9 (- (.x _returnvalue_2) _returnvalue_4))
  (bind _returnvalue_10 (+ (.x _returnvalue_2) _returnvalue_4))
  (bind _returnvalue_11 (- (.y _returnvalue_2) _returnvalue_5))
  (bind _returnvalue_12 (+ (.y _returnvalue_2) _returnvalue_5))
  (bind _returnvalue_13 (Math|Random|RandomFloatinRange _returnvalue_7 _returnvalue_8))
  (bind _returnvalue_14 (Math|Random|RandomFloatinRange _returnvalue_9 _returnvalue_10))
  (bind _returnvalue_15 (Math|Random|RandomFloatinRange _returnvalue_11 _returnvalue_12))
  (for _index (range 0 (Variables|Default|GetNumber))
    (if (Variables|Default|GetIsDamagable?)
      (Game|SpawnActorfromClass "/Game/Props/BP_DamagableBox.BP_DamagableBox_C" (Math|Transform|MakeTransform (Math|Vector|MakeVector _returnvalue_14 _returnvalue_15 _returnvalue_13) _returnvalue _scale) "AdjustIfPossibleButAlwaysSpawn" 0 0)
      (else
        (Game|SpawnActorfromClass "/Game/Props/BP_NonDamagableBox.BP_NonDamagableBox_C" (Math|Transform|MakeTransform (Math|Vector|MakeVector _returnvalue_14 _returnvalue_15 _returnvalue_13) _returnvalue _scale) "AdjustIfPossibleButAlwaysSpawn" 0 0)))))

(event Collision|EventActorBeginOverlap
  (params (OtherActor :type Actor%20Object%20Reference)))

(event EventTick
  (params (DeltaSeconds :type Float%20%28single-precision%29)))

(fn ConstructionScript)