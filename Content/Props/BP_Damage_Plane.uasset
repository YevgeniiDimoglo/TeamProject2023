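; BP_Damage_Plane is a hazard prop that damages and knocks back the first-person player on contact.
; On Hit, a player character takes damage and a strong movement impulse along the hit normal.
; A hit from a Rocket Punch passes reduced damage and the same impulse back to its owning player.
; Each Tick sets the Niagara SpriteFacing vector to the actor's up vector, so sprites follow the plane's orientation.
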(event EventBeginPlay)

(event Collision|EventActorBeginOverlap
  (params (OtherActor :type Actor%20Object%20Reference)))

(event EventTick
  (params (DeltaSeconds :type Float%20%28single-precision%29))
  (Niagara|SetNiagaraVariable(Vector3) (Variables|Default|GetNiagara) "SpriteFacing" (Transformation|GetActorUpVector)))

(event Collision|EventHit
  (params (MyComp :type Primitive%20Component%20Object%20Reference) (Other :type Actor%20Object%20Reference) (OtherComp :type Primitive%20Component%20Object%20Reference) (bSelfMoved :type Boolean) (HitLocation :type Vector :default "0, 0, 0") (HitNormal :type Vector :default "0, 0, 0") (NormalImpulse :type Vector :default "0, 0, 0") (Hit :type Hit%20Result%20Structure%20%28by%20ref%29))
  (bind _returnvalue (* HitNormal 1e+04))
  (bind _asbp_first_person_character (Utilities|Casting|CastToBP_FirstPersonCharacter Other)
    (:then
      (Default|TakeDamage _asbp_first_person_character 2e+01)
      (Physics|AddImpulse (Variables|/Script/Engine.Character|GetCharacterMovement _asbp_first_person_character) _returnvalue false))
    (:CastFailed
      (bind _asbp_rocket_punch (Utilities|Casting|CastToBP_Rocket_Punch Other))
      (bind _asbp_first_person_character_2 (Utilities|Casting|CastToBP_FirstPersonCharacter (Variables|/Game/Blueprints/BP_Rocket_Punch.BP_Rocket_Punch_C|GetPlayerCharacter _asbp_rocket_punch)))
      (Default|TakeDamage _asbp_first_person_character_2 1e+01)
      (Physics|AddImpulse (Variables|/Script/Engine.Character|GetCharacterMovement _asbp_first_person_character_2) _returnvalue false))))

(fn ConstructionScript)