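; Boss black hole prop that escalates in stages through LevelUp, from growing attraction to a reversed, repelling phase.
; LevelUp sets Force and updates the Niagara effect, enables linked switches at the first stage, and spawns randomly oriented beams in the reversed stages.
; While Force is nonzero, Tick pushes and rotates the player along the hole's axis and sets mass-scaled tangential velocities on "Movable"-tagged meshes, swirling them around it.
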(event EventBeginPlay)

(event Collision|EventActorBeginOverlap
  (params (OtherActor :type Actor%20Object%20Reference)))

(event EventTick
  (params (DeltaSeconds :type Float%20%28single-precision%29))
  (if (!= (Variables|Default|GetForce) 0.0)
    (CallFunction|ForcetoPlayer)
    (CallFunction|ForcetoObject)))

(fn ConstructionScript)

(fn LevelUp
  (bind _niagara (Variables|Default|GetNiagara))
  (bind _result (Math|Integer|IncrementInt (Variables|Default|GetLevel))
    (:%20%20
      (switch int _result
        (:1
          (Class|NiagaraComponent|SetAsset (Variables|Default|GetNiagara) "/Game/Effects/NS_BlackHole.NS_BlackHole" true)
          (for _array_element (Variables|Default|GetSwitches)
            (bind _asbp_pc_black_hole_swtch (Utilities|Casting|CastToBP_PC_BlackHole_Swtch _array_element))
            (Variables|/Game/Props/BP_PC_BlackHole_Swtch.BP_PC_BlackHole_Swtch_C|SetEnable _asbp_pc_black_hole_swtch true)
            (Variables|Default|SetForce 3e+04)))
        (:2
          (Variables|Default|SetForce 5e+04)
          (Niagara|SetNiagaraVariable(Float) _niagara "LifeTime" 2.0)
          (Niagara|SetNiagaraVariable(Float) _niagara "Scale" 2e+01))
        (:3
          (Variables|Default|SetForce 8e+04))
        (:4
          (Variables|Default|SetForce -5e+04)
          (Class|NiagaraComponent|SetAsset (Variables|Default|GetNiagara) "/Game/Effects/NS_BlackHole_Reverse.NS_BlackHole_Reverse" true)
          (for _index (range 0 4) :!label _label
            (CallFunction|NewBeam)))
        (:5
          (Variables|Default|SetForce -8e+04)
          (goto _label))))))

(fn NewBeam
  (Game|SpawnActorfromClass "/Game/Blueprints/BP_Electric_Beam.BP_Electric_Beam_C" (Math|Transform|MakeTransform (Transformation|GetActorLocation) (Math|Random|RandomRotator true)) "Undefined" 0 0))

(fn ForcetoPlayer
  (bind _returnvalue (Game|GetPlayerCharacter 0))
  (bind _returnvalue_2 (Transformation|GetActorLocation))
  (bind _returnvalue_3 (Transformation|GetActorLocation _returnvalue))
  (bind _returnvalue_4 (Math|Vector|GetUnitDirection(Vector) _returnvalue_3 _returnvalue_2))
  (bind _asbp_first_person_character (Utilities|Casting|CastToBP_FirstPersonCharacter _returnvalue))
  (Physics|AddForce (Variables|/Script/Engine.Character|GetCharacterMovement _returnvalue) (* _returnvalue_4 (Variables|Default|GetForce)))
  (Default|RotatePlayer _asbp_first_person_character (* (CallFunction|RotatorfromTwoVectors (Math|Vector|NegateVector (Transformation|GetActorUpVector _returnvalue)) _returnvalue_4) 0.005)))

(fn ForcetoObject
  (bind _outactors (Actor|GetAllActorswithTag "Movable"))
  (for _array_element _outactors
    (Physics|SetPhysicsLinearVelocity (Actor|GetComponentbyClass _array_element "/Script/Engine.StaticMeshComponent") (/ (* (Math|Vector|CrossProduct (Math|Vector|VectorUp) (Math|Vector|GetUnitDirection(Vector) (Transformation|GetActorLocation _array_element) (Transformation|GetActorLocation))) (Variables|Default|GetForce) 1e+02) (Physics|GetMass (Actor|GetComponentbyClass _array_element "/Script/Engine.StaticMeshComponent"))) false "None")))