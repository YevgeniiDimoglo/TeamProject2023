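; BP_PC_BlackHole_Swtch is a PC monitor switch prop that levels up the black hole boss when struck by a rocket punch.
; While enabled, Tick shows a click marker when the player is within active distance, or a location widget fed the switch's position when farther away.
; A rocket punch hit in range disables the switch, changes its monitor material to light blue, and calls LevelUp on BP_Boss_BlackHole.
; EnableSwitch re-arms it.
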(event EventBeginPlay
  (bind _asw_location (Utilities|Casting|CastToW_Location (UserInterface|GetWidget (Variables|Default|GetClick_Location))))
  (Variables|/Game/Widget/W_Location.W_Location_C|SetOriginLocation _asw_location (Transformation|GetActorLocation)))

(event Collision|EventActorBeginOverlap
  (params (OtherActor :type Actor%20Object%20Reference)))

(event Collision|EventHit
  (params (MyComp :type Primitive%20Component%20Object%20Reference) (Other :type Actor%20Object%20Reference) (OtherComp :type Primitive%20Component%20Object%20Reference) (bSelfMoved :type Boolean) (HitLocation :type Vector :default "0, 0, 0") (HitNormal :type Vector :default "0, 0, 0") (NormalImpulse :type Vector :default "0, 0, 0") (Hit :type Hit%20Result%20Structure%20%28by%20ref%29))
  (if (Variables|Default|GetEnable)
    (if (<= (CallFunction|PlayerDistance) (Variables|Default|GetActiveDistance))
      (Utilities|Casting|CastToBP_Rocket_Punch Other)
      (CallFunction|SwitchPress))))

(event EventTick
  (params (DeltaSeconds :type Float%20%28single-precision%29))
  (if (Variables|Default|GetEnable)
    (if (<= (CallFunction|PlayerDistance) (Variables|Default|GetActiveDistance))
      (Rendering|SetVisibility (Variables|Default|GetClick_Maker) true false)
      (Rendering|SetVisibility (Variables|Default|GetClick_Location) false false)
      (else
        (Rendering|SetVisibility (Variables|Default|GetClick_Maker) false false)
        (Rendering|SetVisibility (Variables|Default|GetClick_Location) true false)))
    (else
      (Rendering|SetVisibility (Variables|Default|GetClick_Maker) false false)
      (Rendering|SetVisibility (Variables|Default|GetClick_Location) false false))))

(fn ConstructionScript)

(fn PlayerDistance
  (return (Math|Vector|Distance(Vector) (Transformation|GetActorLocation (Game|Player|GetPlayerPawn 0)) (Transformation|GetActorLocation))))

(fn SwitchPress
  (Variables|Default|SetEnable false)
  (Rendering|Material|SetMaterial (Variables|Default|GetSM_monitor) 0 "/Game/Materials/M_Emssive_Light_Blue.M_Emssive_Light_Blue")
  (bind _asbp_boss_black_hole (Utilities|Casting|CastToBP_Boss_BlackHole (Variables|Default|GetBlackHole)))
  (Default|LevelUp _asbp_boss_black_hole))

(fn EnableSwitch
  (Variables|Default|SetEnable true))