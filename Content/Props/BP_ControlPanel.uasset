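; BP_ControlPanel is a one-shot control panel prop whose screen starts red and turns green once activated.
; The first overlap of its Box by any component calls StartInteraction on BPInteraction, swaps the screen material and latches IsActivated.
; Tick shows ClickMaker only while the panel is inactive and the player pawn is within ActiveDistance.
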(event OnComponentBeginOverlap(Box)
  (params (OverlappedComponent :type Primitive%20Component%20Object%20Reference) (OtherActor :type Actor%20Object%20Reference) (OtherComp :type Primitive%20Component%20Object%20Reference) (OtherBodyIndex :type Integer) (bFromSweep :type Boolean) (SweepResult :type Hit%20Result%20Structure%20%28by%20ref%29))
  (if (not (Variables|Default|GetIsActivated?))
    (Default|StartInteraction (Variables|Default|GetBP_Interaction))
    (Rendering|Material|SetMaterial (Variables|Default|GetCP_screen) 0 "/Game/Models/ControlPanel/Materials/M_GreenLight.M_GreenLight")
    (Variables|Default|SetIsActivated? true)))

(event EventBeginPlay)

(event Collision|EventActorBeginOverlap
  (params (OtherActor :type Actor%20Object%20Reference)))

(event EventTick
  (params (DeltaSeconds :type Float%20%28single-precision%29))
  (if (Variables|Default|GetIsActivated?)
    (Rendering|SetVisibility (Variables|Default|GetClick_Maker) false false)
    (elif (<= (Math|Vector|Distance(Vector) (Transformation|GetActorLocation (Game|Player|GetPlayerPawn 0)) (Transformation|GetActorLocation)) (Variables|Default|GetActiveDistance))
      (Rendering|SetVisibility (Variables|Default|GetClick_Maker) true false)
      (else
        (Rendering|SetVisibility (Variables|Default|GetClick_Maker) false false)))))

(fn ConstructionScript
  (Rendering|Material|SetMaterial (Variables|Default|GetCP_screen) 0 "/Game/Models/ControlPanel/Materials/M_RedLight.M_RedLight"))