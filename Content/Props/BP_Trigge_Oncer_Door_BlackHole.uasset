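; One-shot trigger actor that opens or closes a linked door and removes a linked black hole.
; Its BeginOverlap function calls CloseDoor or OpenDoor on the Door reference according to the Close flag.
; It then destroys the BlackHole actor and itself, so the trigger works only once.
; The event graph holds only disabled default events.
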(event EventBeginPlay
  (|CallParentFunction) ; このノードは無効になっているため呼び出せません。\n機能をビルドするにはピンをドラッグしてください。
)

(event Collision|EventActorBeginOverlap
  (params (OtherActor :type Actor%20Object%20Reference))
  (|CallParentFunction OtherActor) ; このノードは無効になっているため呼び出せません。\n機能をビルドするにはピンをドラッグしてください。
)

(event EventTick
  (params (DeltaSeconds :type Float%20%28single-precision%29))
  (|CallParentFunction DeltaSeconds) ; このノードは無効になっているため呼び出せません。\n機能をビルドするにはピンをドラッグしてください。
)

(fn ConstructionScript
  (|CallParentFunction))

(fn BeginOverlap
  (bind _door (Variables|Default|GetDoor))
  (if (Variables|Default|GetClose)
    (Default|CloseDoor _door)
    (else
      (Default|OpenDoor _door)))
  (Actor|DestroyActor (Variables|Default|GetBlackHole))
  (Actor|DestroyActor))