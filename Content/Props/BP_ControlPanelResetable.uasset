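; BP_ControlPanelResetable is a control panel prop that resets itself after being triggered by an overlap.
; It extends a parent panel, running the parent's overlap logic first and then waiting for Duration.
; After the delay it sets the CPScreen material back to M_RedLight and clears IsActivated.
; The child does not filter the overlapping actor before starting the reset.
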(event EventBeginPlay
  (|CallParentFunction) ; This node is disabled and will not be called.\nDrag off pins to build functionality.
)

(event Collision|EventActorBeginOverlap
  (params (OtherActor :type Actor%20Object%20Reference))
  (|CallParentFunction OtherActor)
  (Utilities|FlowControl|Delay (Variables|Default|GetDuration))
  (Rendering|Material|SetMaterial (Variables|Default|GetCP_screen) 0 "/Game/Models/ControlPanel/Materials/M_RedLight.M_RedLight")
  (Variables|Default|SetIsActivated? false))

(event EventTick
  (params (DeltaSeconds :type Float%20%28single-precision%29))
  (|CallParentFunction DeltaSeconds) ; This node is disabled and will not be called.\nDrag off pins to build functionality.
)

(fn ConstructionScript
  (|CallParentFunction))