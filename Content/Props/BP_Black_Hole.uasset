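; Black hole prop that pulls the first-person player and "Movable"-tagged actors within Range toward its center.
; Each Tick it scans every actor in the level, applying a constant Force through character movement for the player or AddForceToActor for tagged actors.
; It also gradually rotates the player so their up vector points away from the hole.
; RadomScale randomizes the Outer and Inner component scales every frame for a flickering look.
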(event EventBeginPlay)

(event Collision|EventActorBeginOverlap
  (params (OtherActor :type Actor%20Object%20Reference)))

(event EventTick
  (params (DeltaSeconds :type Float%20%28single-precision%29))
  (bind _returnvalue (Transformation|GetActorLocation))
  (CallFunction|RadomScale)
  (bind _outactors (Actor|GetAllActorsOfClass "/Script/Engine.Actor"))
  (for _array_element _outactors
    (if (< (Math|Vector|Distance(Vector) (Transformation|GetActorLocation _array_element) _returnvalue) (Variables|Default|GetRange))
      (bind _asbp_first_person_character (Utilities|Casting|CastToBP_FirstPersonCharacter _array_element)
        (:then
          (Physics|AddForce (Variables|/Script/Engine.Character|GetCharacterMovement _asbp_first_person_character) (* (Math|Vector|GetUnitDirection(Vector) (Transformation|GetActorLocation _array_element) _returnvalue) (Variables|Default|GetForce)))
          (Default|RotatePlayer _asbp_first_person_character (* (CallFunction|RotatorfromTwoVectors (Transformation|GetActorUpVector _asbp_first_person_character) (Math|Vector|NegateVector (Math|Vector|GetUnitDirection(Vector) (Transformation|GetActorLocation _array_element) _returnvalue))) 0.005)))
        (:CastFailed
          (if (Actor|ActorHasTag _array_element "Movable")
            (CallFunction|AddForcetoActor _array_element (* (Math|Vector|GetUnitDirection(Vector) (Transformation|GetActorLocation _array_element) _returnvalue) (Variables|Default|GetForce)))))))))

(fn ConstructionScript)

(fn RadomScale
  (bind _returnvalue (Math|Random|RandomFloatinRange 0.9 1.0))
  (bind _returnvalue_2 (Math|Random|RandomFloatinRange 1.5 2.0))
  (Transformation|SetRelativeScale3D (Variables|Default|GetOuter) (Math|Vector|MakeVector _returnvalue_2 _returnvalue_2 _returnvalue_2))
  (Transformation|SetRelativeScale3D (Variables|Default|GetInner) (Math|Vector|MakeVector _returnvalue _returnvalue _returnvalue)))