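; Laser hazard that a linked Trigger actor's interaction component switches off for a set Duration before it reactivates.
; Deactivate and Activate toggle laser visibility, mesh collision and an IsSafe flag.
; While unsafe, box overlap damages the first-person character and knocks it back against its velocity.
; An overlapping Rocket Punch instead damages the player character more heavily, without knockback.
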(event OnComponentBeginOverlap(Box)
  (params (OverlappedComponent :type Primitive%20Component%20Object%20Reference) (OtherActor :type Actor%20Object%20Reference) (OtherComp :type Primitive%20Component%20Object%20Reference) (OtherBodyIndex :type Integer) (bFromSweep :type Boolean) (SweepResult :type Hit%20Result%20Structure%20%28by%20ref%29))
  (bind _asbp_first_person_character (Utilities|Casting|CastToBP_FirstPersonCharacter OtherActor)
    (:then
      (if (not (Variables|Default|GetIsSafe?))
        (Default|TakeDamage _asbp_first_person_character 3e+01)
        (Physics|AddImpulse (Variables|/Script/Engine.Character|GetCharacterMovement _asbp_first_person_character) (* (Math|Vector|NegateVector (Math|Vector|Normalize (Transformation|GetVelocity OtherActor))) 2e+05) false)))
    (:CastFailed
      (Utilities|Casting|CastToBP_Rocket_Punch OtherActor)
      (if (not (Variables|Default|GetIsSafe?))
        (bind _asbp_first_person_character_2 (Utilities|Casting|CastToBP_FirstPersonCharacter (Game|GetPlayerCharacter 0)))
        (Default|TakeDamage _asbp_first_person_character_2 5e+01)))))

(event Custom|Deactivate
  (for _array_element (Components|GetChildrenComponents (Variables|Default|GetLasers) false)
    (Rendering|SetVisibility _array_element false false)
    (Collision|SetCollisionEnabled (Variables|Default|GetStaticMesh) "NoCollision")
    (Variables|Default|SetIsSafe? true)))

(event Custom|OnInteract_Event
  (params (on :type Boolean))
  (if on
    (CallFunction|Deactivate)
    (Utilities|FlowControl|Delay (Variables|Default|GetDuration))
    (CallFunction|Activate)))

(event Custom|Activate
  (for _array_element (Components|GetChildrenComponents (Variables|Default|GetLasers) false)
    (Rendering|SetVisibility _array_element true false)
    (Collision|SetCollisionEnabled (Variables|Default|GetStaticMesh) "QueryAndPhysics")
    (Variables|Default|SetIsSafe? false)))

(event EventBeginPlay
  (bind _trigger (Variables|Default|GetTrigger)
    (:then
      (Utilities|IsValid (Actor|GetComponentbyClass _trigger "/Game/Blueprints/BP_Interaction.BP_Interaction_C")
        (:Is%20Valid
          (EventDispatchers|AssignOnInteract (Actor|GetComponentbyClass _trigger "/Game/Blueprints/BP_Interaction.BP_Interaction_C") (delegate Custom|OnInteract_Event)))))
    (:else)))

(event Collision|EventActorBeginOverlap
  (params (OtherActor :type Actor%20Object%20Reference)))

(event EventTick
  (params (DeltaSeconds :type Float%20%28single-precision%29)))

(fn ConstructionScript)