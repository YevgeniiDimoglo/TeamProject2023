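; BP_Laser is a timed laser hazard that switches on and off on a looping timer, started after a configurable offset.
; Each toggle flips IsSafe, the Block component's collision and the visibility of the Scene component's children.
; While active, Box overlaps damage the first-person character and shove it against its velocity.
; An overlapping BP_Rocket_Punch instead deals lighter damage to the player character.
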(event OnComponentBeginOverlap(Box)
  (params (OverlappedComponent :type Primitive%20Component%20Object%20Reference) (OtherActor :type Actor%20Object%20Reference) (OtherComp :type Primitive%20Component%20Object%20Reference) (OtherBodyIndex :type Integer) (bFromSweep :type Boolean) (SweepResult :type Hit%20Result%20Structure%20%28by%20ref%29))
  (bind _asbp_first_person_character (Utilities|Casting|CastToBP_FirstPersonCharacter OtherActor)
    (:then
      (if (not (Variables|Default|GetIsSafe?))
        (Default|TakeDamage _asbp_first_person_character 5e+01)
        (Physics|AddImpulse (Variables|/Script/Engine.Character|GetCharacterMovement _asbp_first_person_character) (* (Math|Vector|NegateVector (Math|Vector|Normalize (Transformation|GetVelocity OtherActor))) 2e+05) false)))
    (:CastFailed
      (Utilities|Casting|CastToBP_Rocket_Punch OtherActor)
      (if (not (Variables|Default|GetIsSafe?))
        (bind _asbp_first_person_character_2 (Utilities|Casting|CastToBP_FirstPersonCharacter (Game|GetPlayerCharacter 0)))
        (Default|TakeDamage _asbp_first_person_character_2 1e+01)))))

(event EventBeginPlay
  (Variables|Default|SetIsSafe? false)
  (Utilities|FlowControl|Delay (Variables|Default|GetTimer%20Offset))
  (Utilities|Time|SetTimerbyFunctionName 0 "DisableHitBox" (Variables|Default|GetTimer%20Lenght) true))

(event Collision|EventActorBeginOverlap
  (params (OtherActor :type Actor%20Object%20Reference)))

(event EventTick
  (params (DeltaSeconds :type Float%20%28single-precision%29)))

(fn ConstructionScript)

(fn DisableHitBox
  (bind _output_get (Variables|Default|SetIsSafe? (select (Variables|Default|GetIsSafe?) false true)))
  (if _output_get
    (Collision|SetCollisionEnabled (Variables|Default|GetBlock) "NoCollision")
    (for _array_element (Components|GetChildrenComponents (Variables|Default|GetScene) false)
      (Rendering|SetVisibility _array_element false false))
    (else
      (Collision|SetCollisionEnabled (Variables|Default|GetBlock) "QueryAndPhysics")
      (for _array_element_2 (Components|GetChildrenComponents (Variables|Default|GetScene) false)
        (Rendering|SetVisibility _array_element_2 true false)))))