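; BP_NewDoor is a double sliding door prop opened by a linked Trigger actor.
; On BeginPlay it binds to the Trigger's BP_Interaction OnInteract event and opens when that reports On.
; A DoorAnimation timeline slides the two leaves apart along local Y, then plays a gate-close sound when finished.
; CloseDoor reverses the timeline but is not called within this Blueprint.
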(event Custom|OpenDoor
  (bind _doormovement (Timeline|DoorAnimation Play)
    (:Update
      (Transformation|SetRelativeLocation (Variables|Default|Getdoor_newset_doorR) (Math|Vector|MakeVector 0.0 (* _doormovement 3.5e+02) 0.0) false false)
      (Transformation|SetRelativeLocation (Variables|Default|Getdoor_newset_doorL) (Math|Vector|MakeVector 0.0 (* _doormovement -3.5e+02) 0.0) false false))
    (:Finished
      (Audio|PlaySoundatLocation "/Game/Sound/SoundEffect/SE_Gate_Close.SE_Gate_Close" (Transformation|GetActorLocation) "0, 0, 0" 1.0 1.0 0.0 "/Game/Sound/SoundAttenuation.SoundAttenuation" 0 0 0))))

(event Custom|CloseDoor
  (bind _doormovement (Timeline|DoorAnimation Reverse)
    (:Update
      (Transformation|SetRelativeLocation (Variables|Default|Getdoor_newset_doorR) (Math|Vector|MakeVector 0.0 (* _doormovement 3.5e+02) 0.0) false false)
      (Transformation|SetRelativeLocation (Variables|Default|Getdoor_newset_doorL) (Math|Vector|MakeVector 0.0 (* _doormovement -3.5e+02) 0.0) false false))
    (:Finished
      (Audio|PlaySoundatLocation "/Game/Sound/SoundEffect/SE_Gate_Close.SE_Gate_Close" (Transformation|GetActorLocation) "0, 0, 0" 1.0 1.0 0.0 "/Game/Sound/SoundAttenuation.SoundAttenuation" 0 0 0))))

(event Custom|OnInteract_Event
  (params (on :type Boolean))
  (if on
    (CallFunction|OpenDoor)))

(event EventBeginPlay
  (bind _trigger (Variables|Default|GetTrigger)
    (:then
      (Utilities|IsValid (Actor|GetComponentbyClass _trigger "/Game/Blueprints/BP_Interaction.BP_Interaction_C")
        (:Is%20Valid
          (EventDispatchers|AssignOnInteract (Actor|GetComponentbyClass _trigger "/Game/Blueprints/BP_Interaction.BP_Interaction_C") (delegate Custom|OnInteract_Event)))))
    (:else)))

(fn ConstructionScript)