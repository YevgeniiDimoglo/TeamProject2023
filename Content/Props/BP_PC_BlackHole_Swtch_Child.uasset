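; Child switch prop for the black hole boss fight: a computer with body, keyboard and monitor hidden in game.
; When hit by a BP_Rocket_Punch while the player is within ActiveDistance, it runs Switch.
; Switch clears Enable, sets the screen to a red or green light based on IsOff, and calls LevelUp on the referenced BP_Boss_BlackHole in both branches.
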(event EventBeginPlay
  (|CallParentFunction))

(event Collision|EventActorBeginOverlap
  (params (OtherActor :type Actor%20Object%20Reference))
  (|CallParentFunction OtherActor))

(event EventTick
  (params (DeltaSeconds :type Float%20%28single-precision%29))
  (|CallParentFunction DeltaSeconds) ; This node is disabled and will not be called.\nDrag off pins to build functionality.
)

(event Collision|EventHit
  (params (MyComp :type Primitive%20Component%20Object%20Reference) (Other :type Actor%20Object%20Reference) (OtherComp :type Primitive%20Component%20Object%20Reference) (bSelfMoved :type Boolean) (HitLocation :type Vector :default "0, 0, 0") (HitNormal :type Vector :default "0, 0, 0") (NormalImpulse :type Vector :default "0, 0, 0") (Hit :type Hit%20Result%20Structure%20%28by%20ref%29))
  (if (<= (CallFunction|PlayerDistance) (Variables|Default|GetActiveDistance))
    (Utilities|Casting|CastToBP_Rocket_Punch Other)
    (CallFunction|Switch)))

(fn ConstructionScript
  (|CallParentFunction)
  (Development|SetHiddeninGame (Variables|Default|GetSM_computer_body) true false)
  (Development|SetHiddeninGame (Variables|Default|GetSM_keyboard) true false)
  (Development|SetHiddeninGame (Variables|Default|GetSM_monitor) true false))

(fn Switch
  (Variables|Default|SetEnable false)
  (if (Variables|Default|GetIsOff?)
    (Rendering|Material|SetMaterial (Variables|Default|GetSM_CP_screen) 0 "/Game/Models/ControlPanel/Materials/M_RedLight.M_RedLight")
    (Variables|Default|SetIsOff? false)
    (bind _asbp_boss_black_hole (Utilities|Casting|CastToBP_Boss_BlackHole (Variables|Default|GetBlackHole)))
    (Default|LevelUp _asbp_boss_black_hole)
    (else
      (Rendering|Material|SetMaterial (Variables|Default|GetSM_CP_screen) 0 "/Game/Models/ControlPanel/Materials/M_GreenLight.M_GreenLight")
      (bind _asbp_boss_black_hole_2 (Utilities|Casting|CastToBP_Boss_BlackHole (Variables|Default|GetBlackHole)))
      (Default|LevelUp _asbp_boss_black_hole_2))))