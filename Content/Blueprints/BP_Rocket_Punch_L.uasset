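; BP_Rocket_Punch_L is the left-hand rocket punch, a child Blueprint that supplies left-side specifics to its parent class.
; OriginPoint returns the player character's left arm point, and OtherHand returns its right rocket punch.
; On destruction it shows the player's left HUD and left hand again and hides the left cable.
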(event EventBeginPlay
  (|CallParentFunction))

(event Collision|EventActorBeginOverlap
  (params (OtherActor :type Actor%20Object%20Reference))
  (|CallParentFunction OtherActor) ; このノードは無効になっているため呼び出せません。\n機能をビルドするにはピンをドラッグしてください。
)

(event EventTick
  (params (DeltaSeconds :type Float%20%28single-precision%29))
  (|CallParentFunction DeltaSeconds) ; このノードは無効になっているため呼び出せません。\n機能をビルドするにはピンをドラッグしてください。
)

(event EventDestroyed
  (bind _playercharacter (Variables|Default|GetPlayerCharacter))
  (Default|SetHUDVisibility _playercharacter true "Visible")
  (Rendering|SetVisibility (Variables|/Game/Blueprints/BP_FirstPersonCharacter.BP_FirstPersonCharacter_C|GetCable_L _playercharacter) false false)
  (Rendering|SetVisibility (Variables|/Game/Blueprints/BP_FirstPersonCharacter.BP_FirstPersonCharacter_C|GetHand_L _playercharacter) true true))

(fn ConstructionScript
  (|CallParentFunction))

(fn OriginPoint
  (bind _arm_point_l (Default|ArmPointLeft (Variables|Default|GetPlayerCharacter)))
  (return _arm_point_l))

(fn OtherHand
  (return (Variables|/Game/Blueprints/BP_FirstPersonCharacter.BP_FirstPersonCharacter_C|GetRocketPunch_R (Variables|Default|GetPlayerCharacter))))