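; Right-hand rocket punch Blueprint, specializing the player's rocket punch for the right arm.
; It overrides OriginPoint to return the player character's right arm point.
; When destroyed, it makes the right-side HUD visible again and hides the player's right cable.
; It adds no active BeginPlay, overlap or Tick logic of its own.
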(event EventBeginPlay
  (|CallParentFunction) ; このノードは無効になっているため呼び出せません。\n機能をビルドするにはピンをドラッグしてください。
)

(event Collision|EventActorBeginOverlap
  (params (OtherActor :type Actor%20Object%20Reference))
  (|CallParentFunction OtherActor) ; このノードは無効になっているため呼び出せません。\n機能をビルドするにはピンをドラッグしてください。
)

(event EventTick
  (params (DeltaSeconds :type Float%20%28single-precision%29))
  (|CallParentFunction DeltaSeconds) ; このノードは無効になっているため呼び出せません。\n機能をビルドするにはピンをドラッグしてください。
)

(event EventDestroyed
  (bind _playercharacter (Variables|Default|GetPlayerCharacter))
  (Default|SetHUDVisibility _playercharacter false "Visible")
  (Rendering|SetVisibility (Variables|/Game/Blueprints/BP_FirstPersonCharacter.BP_FirstPersonCharacter_C|GetCable_R _playercharacter) false false))

(fn ConstructionScript
  (|CallParentFunction))

(fn OriginPoint
  (bind _arm_point_l (Default|ArmPointRight (Variables|Default|GetPlayerCharacter)))
  (return _arm_point_l))