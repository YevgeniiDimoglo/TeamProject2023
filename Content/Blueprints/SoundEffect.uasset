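; SoundEffect is a set of helper functions that play the game's UI, damage and gate sound effects.
; UI console, select and cancel sounds go through InstancePlaySound, which casts the game instance to MyGameInstance and forwards playback to it.
; The damage sound plays directly in 2D, while the gate-close sound plays at a given location with attenuation and caller-set volume, pitch and start time.
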(fn InstancePlaySound
  (params (Sound :type Sound%20Base%20Object%20Reference) (Volume :type Float%20%28double-precision%29) (Pitch :type Float%20%28double-precision%29) (StartTime :type Float%20%28double-precision%29))
  (bind _asmy_game_instance (Utilities|Casting|CastToMyGameInstance (Game|GetGameInstance)))
  (Default|InstancePlaySound _asmy_game_instance Sound Volume Pitch StartTime))

(fn UISoundConsole
  (CallFunction|InstancePlaySound "/Game/Sound/SoundEffect/SE_Console.SE_Console" 1.0 1.0 0.0))

(fn UISoundSelect
  (CallFunction|InstancePlaySound "/Game/Sound/SoundEffect/SE_Select.SE_Select" 1.0 1.0 0.0))

(fn UISoundCancel
  (CallFunction|InstancePlaySound "/Game/Sound/SoundEffect/SE_Cancel.SE_Cancel" 1.0 1.0 0.0))

(fn SoundDamage
  (Audio|PlaySound2D 0 "/Game/Sound/SoundEffect/SE_Damage.SE_Damage" 1.0 1.0 0.0 0 0))

(fn SoundGate
  (params (Location :type Vector) (Volume :type Float%20%28double-precision%29) (Pitch :type Float%20%28double-precision%29) (StartTime :type Float%20%28double-precision%29))
  (Audio|PlaySoundatLocation 0 "/Game/Sound/SoundEffect/SE_Gate_Close.SE_Gate_Close" Location "0, 0, 0" Volume Pitch StartTime "/Game/Sound/SoundAttenuation.SoundAttenuation" 0 0 0))