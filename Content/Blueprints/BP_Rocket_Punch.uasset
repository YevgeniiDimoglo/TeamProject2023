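; Rocket punch projectile that works as a grappling hook for the first-person character.
; It attaches to "Grappable" hits; other hits or exceeding ArmLength release it to fly back to OriginPoint and self-destroy.
; PullObject starts per-tick forces drawing the player toward the fist, with opposite force on "Movable" targets.
; Distances and directions use OriginPoint, which returns a fixed zero vector here.
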(event EventBeginPlay
  (bind _asbp_first_person_character (Utilities|Casting|CastToBP_FirstPersonCharacter (Game|GetPlayerCharacter 0)))
  (Variables|Default|SetPlayerCharacter _asbp_first_person_character))

(event Collision|EventActorBeginOverlap
  (params (OtherActor :type Actor%20Object%20Reference)))

(event EventTick
  (params (DeltaSeconds :type Float%20%28single-precision%29))
  (bind _returnvalue (Transformation|GetActorLocation))
  (bind _point (CallFunction|OriginPoint))
  (bind _returnvalue_2 (Math|Vector|Distance(Vector) _returnvalue _point))
  (if (Variables|Default|Getenable)
    (if (> _returnvalue_2 (Variables|/Game/Blueprints/BP_FirstPersonCharacter.BP_FirstPersonCharacter_C|GetArmLength (Variables|Default|GetPlayerCharacter)))
      (CallFunction|ReleaseGrab)
      (if (< _returnvalue_2 1e+02) :!label _label
        (Actor|DestroyActor)
        (else
          (Variables|/Script/Engine.MovementComponent|SetVelocity (Variables|MyProjectile|GetProjectileMovement) (* (Math|Vector|Normalize (Math|Vector|GetUnitDirection(Vector) (Transformation|GetActorLocation) (CallFunction|OriginPoint))) 1e+04))))
      (elif (Variables|Default|GetPulling)
        (CallFunction|PullingUpdate)))
    (else
      (goto _label))))

(event Collision|EventHit
  (params (MyComp :type Primitive%20Component%20Object%20Reference) (Other :type Actor%20Object%20Reference) (OtherComp :type Primitive%20Component%20Object%20Reference) (bSelfMoved :type Boolean) (HitLocation :type Vector :default "0, 0, 0") (HitNormal :type Vector :default "0, 0, 0") (NormalImpulse :type Vector :default "0, 0, 0") (Hit :type Hit%20Result%20Structure%20%28by%20ref%29))
  (if (and (Variables|Default|Getenable) (not (Variables|Default|GetGrapping)))
    (if (Actor|ActorHasTag Other "Grappable")
      (Variables|Default|SetGrapping true)
      (Components|Movement|StopMovementImmediately (Variables|MyProjectile|GetProjectileMovement))
      (Transformation|AttachActorToActor Other "None" "KeepWorld" "KeepWorld" "KeepWorld" true)
      (Variables|Default|SetGrappedObject Other)
      (else
        (CallFunction|ReleaseGrab)))))

(fn ConstructionScript)

(fn ReleaseGrab
  (Variables|Default|Setenable false)
  (Variables|Default|SetGrapping false)
  (Variables|Default|SetPulling false)
  (Transformation|DetachFromActor "KeepWorld" "KeepWorld" "KeepWorld")
  (Collision|SetCollisionEnabled (Variables|Default|GetPunch) "NoCollision"))

(fn PullObject
  (Variables|Default|SetPulling true))

(fn OriginPoint
  (return "0, 0, 0"))

(fn PullingUpdate
  (bind _point (CallFunction|OriginPoint))
  (bind _returnvalue (Transformation|GetActorLocation))
  (bind _playercharacter (Variables|Default|GetPlayerCharacter))
  (bind _pullingforce (Variables|Default|GetPullingForce))
  (bind _grappedobject (Variables|Default|GetGrappedObject))
  (bind _returnvalue_2 (Math|Vector|GetUnitDirection(Vector) _point _returnvalue))
  (bind _charactermovement (Variables|/Script/Engine.Character|GetCharacterMovement _playercharacter))
  (bind _returnvalue_3 (* _returnvalue_2 _pullingforce))
  (bind _returnvalue_4 (* _returnvalue_3 -1.0))
  (if (< (Math|Vector|Distance(Vector) _point _returnvalue) 75.0)
    (Components|Movement|StopMovementImmediately _charactermovement))
  (Physics|AddForce _charactermovement _returnvalue_3)
  (if (Actor|ActorHasTag _grappedobject "Movable")
    (bind _asbp_movable (Utilities|Casting|CastToBP_Movable _grappedobject)
      (:then
        (Class|PrimitiveComponent|AddForceatLocation (Variables|/Script/Engine.StaticMeshActor|GetStaticMeshComponent _asbp_movable) _returnvalue_4 _returnvalue "None"))
      (:CastFailed
        (for _array_element (Actor|GetComponentsByClass _grappedobject "/Script/Engine.StaticMeshComponent")
          (Class|PrimitiveComponent|AddForceatLocation _array_element _returnvalue_4 _returnvalue "None"))))))