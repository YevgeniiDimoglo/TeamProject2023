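; BP_Teleport is a trigger actor that plays a short transition and then loads another level.
; When BP_FirstPersonCharacter enters the Box, it disables player input, hides the character and removes all widgets.
; It spawns an enlarged BP_NYaNC022 at SpawnPoint as a stand-in model and blends the view to itself.
; After a delay matching the blend time, it opens the level named by LevelName.
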(event OnComponentBeginOverlap(Box)
  (params (OverlappedComponent :type Primitive%20Component%20Object%20Reference) (OtherActor :type Actor%20Object%20Reference) (OtherComp :type Primitive%20Component%20Object%20Reference) (OtherBodyIndex :type Integer) (bFromSweep :type Boolean) (SweepResult :type Hit%20Result%20Structure%20%28by%20ref%29))
  (bind _returnvalue (Game|GetPlayerController 0))
  (bind _asbp_first_person_character (Utilities|Casting|CastToBP_FirstPersonCharacter OtherActor))
  (Input|DisableInput _returnvalue 0)
  (Rendering|SetActorHiddenInGame _asbp_first_person_character true)
  (Viewport|RemoveAllWidgets)
  (bind _returnvalue_2 (Game|SpawnActorfromClass "/Game/Props/BP_NYaN-C0-22.BP_NYaN-C0-22_C" (Transformation|GetWorldTransform (Variables|Default|GetSpawnPoint)) "Undefined" 0 0))
  (bind _output_get (Variables|Default|SetNewCharacterModel _returnvalue_2))
  (Transformation|SetActorScale3D _output_get "10.000000,10.000000,10.000000")
  (Game|Player|SetViewTargetwithBlend _returnvalue self 5.0 "VTBlend_Linear" 0.0 false)
  (Utilities|FlowControl|Delay 5.0)
  (Game|OpenLevel(byName) (Variables|Default|GetLevel%20Name)))

(event EventBeginPlay)

(event Collision|EventActorBeginOverlap
  (params (OtherActor :type Actor%20Object%20Reference)))

(event EventTick
  (params (DeltaSeconds :type Float%20%28single-precision%29)))

(fn ConstructionScript)