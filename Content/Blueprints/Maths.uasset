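; Maths is a Blueprint collection of helper functions for vector rotation math and whole-actor physics.
; Vector helpers give the direction between actors, the angle via acos of the dot product without normalizing inputs, and an axis-angle rotator from the cross product.
; Physics helpers loop over an actor's primitive components to sum the mass of simulating ones, toggle simulation, or apply the full force to each.
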(fn RotatorfromTwoVectors
  (params (From :type Vector) (To :type Vector))
  (return (Math|Vector|RotatorfromAxisandAngle (Math|Vector|CrossProduct From To) (CallFunction|AngleBetweenVectors From To true))))

(fn AngleBetweenVectors
  (params (From :type Vector) (To :type Vector) (Degree :type Boolean))
  (bind _returnvalue (Math|Vector|DotProduct From To))
  (if (Utilities|Operators|EqualEqual From To 0.0)
    (return 0.0)
    (elif Degree
      (return (Class|KismetMathLibrary|DegAcos _returnvalue))
      (else
        (return (Math|Trig|Acos(Degrees) _returnvalue))))))

(fn GetActorMass
  (params (Actor :type Actor%20Object%20Reference))
  (for _array_element (Actor|GetComponentsByClass Actor "/Script/Engine.PrimitiveComponent")
    (if (Physics|IsSimulatingPhysics _array_element "None")
      (LocalVariables|Setresult (+ (LocalVariables|Getresult) (Physics|GetMass _array_element)))))
  (return (LocalVariables|Getresult)))

(fn DirectionBetweenActors
  (params (From :type Actor%20Object%20Reference) (To :type Actor%20Object%20Reference))
  (return (Math|Vector|GetUnitDirection(Vector) (Transformation|GetActorLocation From) (Transformation|GetActorLocation To))))

(fn SetActorSimulatePhysics
  (params (Actor :type Actor%20Object%20Reference) (SimulatePhysics :type Boolean))
  (for _array_element (Actor|GetComponentsByClass Actor "/Script/Engine.PrimitiveComponent")
    (Physics|SetSimulatePhysics _array_element SimulatePhysics)))

(fn AddForcetoActor
  (params (Actor :type Actor%20Object%20Reference) (Force :type Vector))
  (for _array_element (Actor|GetComponentsByClass Actor "/Script/Engine.PrimitiveComponent")
    (Physics|AddForce _array_element Force "None" false)))