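; LevelFunction is a set of level flow helpers for loading transitions, respawning and resetting.
; BeginLevelLoading starts a WB_Transition widget with min and max load times, skipped when the options string holds Reset=1.
; EndLevel adds a new transition widget to the viewport.
; Respawn and ResetLevel reopen the current level with Reset=1, with Respawn also passing a Checkpoint flag.
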(fn BeginLevelLoading
  (params (PlayerController :type Player%20Controller%20Object%20Reference) (RmdLoadTimeMin :type Float%20%28double-precision%29) (RmdLoadTimeMax :type Float%20%28double-precision%29))
  (if (not (Utilities|Enum|Equal(Enum) (Class|GameplayStatics|ParseOption (Variables|/Script/Engine.GameModeBase|GetOptionsString (Game|GetGameMode)) "Reset") "1"))
    (bind _returnvalue (UserInterface|CreateWidget "/Game/UI/WB_Transition.WB_Transition_C" PlayerController))
    (Default|BeginLevel _returnvalue RmdLoadTimeMin RmdLoadTimeMax)))

(fn EndLevel
  (params (PlayerController :type Player%20Controller%20Object%20Reference))
  (bind _returnvalue (UserInterface|CreateWidget "/Game/UI/WB_Transition.WB_Transition_C" PlayerController))
  (UserInterface|Viewport|AddtoViewport _returnvalue 0))

(fn Respawn
  (bind _returnvalue (Game|GetCurrentLevelName 0))
  (Game|OpenLevel(byName) 0 (Utilities|String|StringToName _returnvalue) true "Reset=1?Checkpoint=1"))

(fn ResetLevel
  (bind _returnvalue (Game|GetCurrentLevelName 0))
  (Game|OpenLevel(byName) 0 (Utilities|String|StringToName _returnvalue) true "Reset=1"))