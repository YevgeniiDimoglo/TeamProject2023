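; A game instance Blueprint that plays 2D sounds and background music and stores the current checkpoint.
; Both play functions create 2D audio components that persist across level transitions, keeping one reference for sound effects and one for BGM.
; StopBGM stops the stored music component if it is valid, and UpdateCheckPoint overwrites the saved checkpoint value.
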(fn InstancePlaySound
  (params (Sound :type Sound%20Base%20Object%20Reference) (Volume :type Float%20%28double-precision%29) (Pitch :type Float%20%28double-precision%29) (StartTime :type Float%20%28double-precision%29))
  (bind _returnvalue (Audio|CreateSound2D Sound Volume Pitch StartTime 0 true))
  (bind _output_get (LocalVariables|SetAudio _returnvalue))
  (Audio|Components|Audio|Play _output_get 0.0))

(fn PlayBGM
  (params (Sound :type Sound%20Base%20Object%20Reference) (Volume :type Float%20%28double-precision%29) (Pitch :type Float%20%28double-precision%29) (StartTime :type Float%20%28double-precision%29))
  (bind _returnvalue (Audio|CreateSound2D Sound Volume Pitch StartTime 0 true))
  (bind _output_get (Variables|Default|SetBGM _returnvalue))
  (Audio|Components|Audio|Play _output_get 0.0))

(fn StopBGM
  (bind _bgm (Variables|Default|GetBGM))
  (if (Utilities|IsValid _bgm)
    (Audio|Components|Audio|Stop _bgm)))

(fn UpdateCheckPoint
  (params (CheckPoint :type Transform))
  (Variables|Default|SetCheckPoint CheckPoint))